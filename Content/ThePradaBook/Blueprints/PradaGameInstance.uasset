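; Game instance that holds the player's money and health and persists them across sessions in a single save slot, loaded on Init.
; Increment and decrement functions update values, notify GameHUD widgets, play a sound and immediately save through a fresh PradaSaveGame object.
; Spending fails when funds are short, and healing is capped at Health.
; DecrementHealth writes its zero-clamped result to Health, leaving CurrentHealth unchanged.
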(event `self.ReceiveInit`
  ;[1 1 1] Load save game on init
  (`self.Load`))

(fn `DecrementHealth`
  (params (Amount :type Integer))
  ;[1 1 1] Decrement health
  (set `self.Health` (`KismetMathLibrary.Max` (- (`self.CurrentHealth`) Amount)))
  (bind _foundwidgets (`WidgetBlueprintLibrary.GetAllWidgetsOfClass` "/Game/ThePradaBook/Widgets/GameHUDWidget.GameHUDWidget_C"))
  (`/Game/ThePradaBook/Widgets/GameHUDWidget.HealthChange` _foundwidgets (`self.CurrentHealth`) (`self.Health`))
  (`GameplayStatics.PlaySound2D` "/Game/ThePradaBook/Sounds/DecrementHealth.DecrementHealth" 1.0 1.0 0.0 null null)
  (`self.Save`))

(fn `DecrementMoney`
  (params (Amount :type Integer))
  (returns (Success :type Boolean))
  (bind _returnvalue (- (`self.Money`) Amount))
  ;[1 1 1] Decrement moeny
  (if (>= _returnvalue 0)
    (set `self.Money` _returnvalue)
    (bind _foundwidgets (`WidgetBlueprintLibrary.GetAllWidgetsOfClass` "/Game/ThePradaBook/Widgets/GameHUDWidget.GameHUDWidget_C"))
    (`/Game/ThePradaBook/Widgets/GameHUDWidget.MoneyChange` _foundwidgets (`self.Money`))
    (`GameplayStatics.PlaySound2D` "/Game/ThePradaBook/Sounds/DecrementMoney.DecrementMoney" 1.0 1.0 0.0 null null)
    (`self.Save`)
    (return true)
    (else
      (return false))))

(fn `IncrementHealth`
  (params (Amount :type Integer))
  ;[1 1 1] Increment health
  (set `self.CurrentHealth` (`KismetMathLibrary.Min` (+ Amount (`self.CurrentHealth`)) (`self.Health`)))
  (bind _foundwidgets (`WidgetBlueprintLibrary.GetAllWidgetsOfClass` "/Game/ThePradaBook/Widgets/GameHUDWidget.GameHUDWidget_C"))
  (`/Game/ThePradaBook/Widgets/GameHUDWidget.HealthChange` _foundwidgets (`self.CurrentHealth`) (`self.Health`))
  (`GameplayStatics.PlaySound2D` "/Game/ThePradaBook/Sounds/IncrementHealth.IncrementHealth" 1.0 1.0 0.0 null null)
  (`self.Save`))

(fn `IncrementMoney`
  (params (Amount :type Integer))
  ;[1 1 1] Increment money
  (set `self.Money` (+ Amount (`self.Money`)))
  (bind _foundwidgets (`WidgetBlueprintLibrary.GetAllWidgetsOfClass` "/Game/ThePradaBook/Widgets/GameHUDWidget.GameHUDWidget_C"))
  (`/Game/ThePradaBook/Widgets/GameHUDWidget.MoneyChange` _foundwidgets (`self.Money`))
  (`GameplayStatics.PlaySound2D` "/Game/ThePradaBook/Sounds/IncrementMoney.IncrementMoney" 1.0 1.0 0.0 null null)
  (`self.Save`))

(fn `Load`
  ;[1 1 1] Load save game
  (bind _returnvalue (`GameplayStatics.LoadGameFromSlot` "DefaultSaveGame"))
  (bind _asprada_save_game (cast `/Game/ThePradaBook/Blueprints/PradaSaveGame` _returnvalue))
  (set `self.Money` (`/Game/ThePradaBook/Blueprints/PradaSaveGame.Money` _asprada_save_game))
  (set `self.Health` (`/Game/ThePradaBook/Blueprints/PradaSaveGame.Health` _asprada_save_game))
  (set `self.CurrentHealth` (`/Game/ThePradaBook/Blueprints/PradaSaveGame.CurrentHealth` _asprada_save_game)))

(fn `Save`
  ;[1 1 1] Save gameinstance to file
  (bind _returnvalue (`GameplayStatics.CreateSaveGameObject` "/Game/ThePradaBook/Blueprints/PradaSaveGame.PradaSaveGame_C"))
  (set `/Game/ThePradaBook/Blueprints/PradaSaveGame.Money` (`self.Money`) _returnvalue)
  (set `/Game/ThePradaBook/Blueprints/PradaSaveGame.Health` (`self.Health`) _returnvalue)
  (set `/Game/ThePradaBook/Blueprints/PradaSaveGame.CurrentHealth` (`self.CurrentHealth`) _returnvalue)
  (`GameplayStatics.SaveGameToSlot` _returnvalue "DefaultSaveGame"))