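; Game mode for story chapters that open with an info screen.
; On BeginPlay it pauses the game, then matches the level path name against Chapter2 through Chapter5 to create that chapter's info widget and add it to the viewport.
; A matched chapter also switches input to Game and UI and shows the mouse cursor; an unmatched level stays paused with no widget.
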(event `self.ReceiveBeginPlay`
  (bind _returnvalue (`GameplayStatics.GetPlayerController` 0))
  (bind _returnvalue_2 (`KismetSystemLibrary.GetPathName` (`self.GetLevel`)))
  ;[1 1 1] Create info widget
  (`GameplayStatics.SetGamePaused` true)
  (if (`KismetStringLibrary.Contains` _returnvalue_2 "Chapter2")
    (bind _returnvalue_3 (`|CreateWidget` "/Game/ThePradaBook/Widgets/Chapter2InfoWidget.Chapter2InfoWidget_C"))
    (`UserWidget.AddToViewport` _returnvalue_3 0)
    (`WidgetBlueprintLibrary.SetInputMode_GameAndUIEx` _returnvalue null "DoNotLock" false :!label _label)
    (set `PlayerController.bShowMouseCursor` true _returnvalue)
    (elif (`KismetStringLibrary.Contains` _returnvalue_2 "Chapter3")
      (bind _returnvalue_4 (`|CreateWidget` "/Game/ThePradaBook/Widgets/Chapter3InfoWidget.Chapter3InfoWidget_C"))
      (`UserWidget.AddToViewport` _returnvalue_4 0)
      (goto _label)
      (elif (`KismetStringLibrary.Contains` _returnvalue_2 "Chapter4")
        (bind _returnvalue_5 (`|CreateWidget` "/Game/ThePradaBook/Widgets/Chapter4InfoWidget.Chapter4InfoWidget_C"))
        (`UserWidget.AddToViewport` _returnvalue_5 0)
        (goto _label)
        (elif (`KismetStringLibrary.Contains` _returnvalue_2 "Chapter5")
          (bind _returnvalue_6 (`|CreateWidget` "/Game/ThePradaBook/Widgets/Chapter5InfoWidget.Chapter5InfoWidget_C"))
          (`UserWidget.AddToViewport` _returnvalue_6 0)
          (goto _label))))))

(fn `UserConstructionScript`)