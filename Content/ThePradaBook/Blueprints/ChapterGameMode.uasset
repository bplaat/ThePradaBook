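; Game mode for the chapter and sandbox levels that opens each level paused with its info widget on screen.
; On BeginPlay it pauses the game, then matches the current level name against Chapter1 through Chapter5 and Sandbox by substring to create the matching widget.
; When a match is found, it sets game-and-UI input and shows the mouse cursor.
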(event `self.ReceiveBeginPlay`
  (bind _returnvalue (`GameplayStatics.GetPlayerController` 0))
  ;[1 1 1] Create info widget
  (`GameplayStatics.SetGamePaused` true)
  (bind _returnvalue_2 (`GameplayStatics.GetCurrentLevelName` true))
  (if (`KismetStringLibrary.Contains` _returnvalue_2 "Chapter1")
    (bind _returnvalue_3 (`|CreateWidget` "/Game/ThePradaBook/Widgets/Chapter1InfoWidget.Chapter1InfoWidget_C"))
    (`UserWidget.AddToViewport` _returnvalue_3 0)
    (`WidgetBlueprintLibrary.SetInputMode_GameAndUIEx` _returnvalue null "DoNotLock" false :!label _label)
    (set `PlayerController.bShowMouseCursor` true _returnvalue)
    (elif (`KismetStringLibrary.Contains` _returnvalue_2 "Chapter2")
      (bind _returnvalue_4 (`|CreateWidget` "/Game/ThePradaBook/Widgets/Chapter2InfoWidget.Chapter2InfoWidget_C"))
      (`UserWidget.AddToViewport` _returnvalue_4 0)
      (goto _label)
      (elif (`KismetStringLibrary.Contains` _returnvalue_2 "Chapter3")
        (bind _returnvalue_5 (`|CreateWidget` "/Game/ThePradaBook/Widgets/Chapter3InfoWidget.Chapter3InfoWidget_C"))
        (`UserWidget.AddToViewport` _returnvalue_5 0)
        (goto _label)
        (elif (`KismetStringLibrary.Contains` _returnvalue_2 "Chapter4")
          (bind _returnvalue_6 (`|CreateWidget` "/Game/ThePradaBook/Widgets/Chapter4InfoWidget.Chapter4InfoWidget_C"))
          (`UserWidget.AddToViewport` _returnvalue_6 0)
          (goto _label)
          (elif (`KismetStringLibrary.Contains` _returnvalue_2 "Chapter5")
            (bind _returnvalue_7 (`|CreateWidget` "/Game/ThePradaBook/Widgets/Chapter5InfoWidget.Chapter5InfoWidget_C"))
            (`UserWidget.AddToViewport` _returnvalue_7 0)
            (goto _label)
            (elif (`KismetStringLibrary.Contains` _returnvalue_2 "Sandbox")
              (bind _returnvalue_8 (`|CreateWidget` "/Game/ThePradaBook/Widgets/SandboxInfoWidget.SandboxInfoWidget_C"))
              (`UserWidget.AddToViewport` _returnvalue_8 0)
              (goto _label))))))))

(fn `UserConstructionScript`)